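; Satisfactory FarmingMod world spawner that scatters pickups of one item class around a list of spawn locations.
; On BeginPlay, it skips any location where a sphere overlap, sized by its Sphere component, finds buildables.
; Elsewhere it counts matching pickups already on the floor and tops them up toward NumberOfDrops.
; New stacks get random amounts and drop in a cylinder around the location.
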(event EventBeginPlay
  (CallFunction|SpawninWorld))

(event Collision|EventActorBeginOverlap
  (params (OtherActor :type Actor%20Object%20Reference)))

(event EventTick
  (params (DeltaSeconds :type Float%20%28single-precision%29)))

(fn ConstructionScript)

(fn SpawninWorld
  (bind _numberofdrops (Variables|Default|GetNumberOfDrops))
  (for _array_element (Variables|Default|GetSpawnLocation)
    (bind _returnvalue (CallFunction|CheckNotinFactory _array_element))
    (if _returnvalue
      (Utilities|Array|Clear (Variables|Default|GetItemArray))
      (bind _items (CallFunction|GetItemsonFloor _array_element))
      (if (not (>= (Utilities|Array|Length _items) _numberofdrops))
        (for _index (range 1 (Math|Integer|Clamp(Integer) (- _numberofdrops (Utilities|Array|Length _items)) 1 _numberofdrops))
          (CallFunction|AddItemtoArray))
        (Class|FGItemPickupSpawnable|CreateItemDropsinCylinder 0 (Variables|Default|GetItemArray) _array_element 1e+03 (Utilities|Array|MakeArray 0) "/Script/FactoryGame.FGItemPickup_Spawnable"))))
  (return))

(fn AddItemtoArray
  (Utilities|Array|Add (Variables|Default|GetItemArray) (Class|FGInventoryLibrary|MakeInventoryStack (Math|Random|RandomIntegerinRange (Variables|Default|GetAmountMin) (Variables|Default|GetAmountMax)) (Class|FGInventoryLibrary|MakeInventoryItem (Variables|Default|GetItemClass))))
  (return))

(fn GetItemsonFloor
  (params (Location :type Vector))
  (bind _outactors (Collision|SphereOverlapActors Location (Variables|/Script/Engine.SphereComponent|GetSphereRadius (Variables|Default|GetSphere)) (Utilities|Array|MakeArray "ObjectTypeQuery1" "ObjectTypeQuery2") "/Script/FactoryGame.FGItemPickup_Spawnable"))
  (for (_array_element _array_index) _outactors
    (bind _asfgitem_pickup_spawnable (Utilities|Casting|CastToFGItemPickup_Spawnable _array_element))
    (if (!= (.out_itemClass (Class|FGInventoryLibrary|BreakInventoryItem (.out_item (Class|FGInventoryLibrary|BreakInventoryStack (Class|FGItemPickup|GetPickupItems _asfgitem_pickup_spawnable))))) (Variables|Default|GetItemClass))
      (Utilities|Array|RemoveIndex _outactors _array_index)))
  (return _outactors))

(fn CheckNotinFactory
  (params (Location :type Vector))
  (bind _returnvalue (Collision|SphereOverlapActors Location (Variables|/Script/Engine.SphereComponent|GetSphereRadius (Variables|Default|GetSphere)) (Utilities|Array|MakeArray "ObjectTypeQuery1" "ObjectTypeQuery2") "/Script/FactoryGame.FGBuildable"))
  (return (not _returnvalue)))